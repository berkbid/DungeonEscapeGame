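; Player controller for a key-collection escape game that owns the HUD, pause menu and game-over flow.
; BeginPlay creates the HUD, and the pause input pauses the game and opens the pause menu.
; UpdateNewKey decrements the key count, updates the HUD and switches the objective to escaping once none remain.
; CallGameOver disables input, sets a pawn lifespan, shows win or loss text and, on a win, destroys the first AI wolf found.
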(event EventBeginPlay
  (bind _returnvalue (UserInterface|CreateWidget "/Game/UI/WBP_PlayerHUD.WBP_PlayerHUD_C" self))
  (bind _output_get (Variables|Default|SetPlayerHUD _returnvalue))
  (UserInterface|Viewport|AddtoViewport _output_get 0))

(event Input|ActionEvents|InputActionPauseGame
  (params (Key :type Key%20Structure :default "None"))
  (:Pressed
    (CallFunction|PauseFunctionality)))

(fn ConstructionScript)

(fn CallGameOver
  (params (bWin :type Boolean))
  (bind _returnvalue (Pawn|GetControlledPawn))
  (bind _self self)
  (bind _self_2 self)
  ;[1 1 1] Disable pawn input and player controller input
  (Input|DisableInput _returnvalue _self_2)
  (Input|DisableInput _self_2 _self_2)
  (Actor|SetLifeSpan _returnvalue 5.0)
  (bind _returnvalue_2 (UserInterface|CreateWidget "/Game/UI/WBP_VictoryMenu.WBP_VictoryMenu_C"))
  (Default|SetVictoryText _returnvalue_2 (Utilities|Select :Index (Math|Integer|SelectInt 0 1 bWin) :Option%200 (Utilities|Text|ToText(String) "Congratulations You Escaped!") :Option%201 (Utilities|Text|ToText(String) "Game Over")))
  (UserInterface|Viewport|AddtoViewport _returnvalue_2 0)
  (Variables|Default|SetbShowMouseCursor _self true)
  (Input|SetInputModeGameandUI _self _returnvalue_2 "DoNotLock" true)
  (if bWin
    (bind _outactors (Actor|GetAllActorsOfClass "/Game/AI/BP_AIWolf.BP_AIWolf_C"))
    (Actor|DestroyActor (Utilities|Array|Get(acopy) _outactors))))

(fn PauseFunctionality
  (bind _self self)
  ;[1 1 1] Pause the game and show pause menu
  (Game|SetGamePaused true)
  (bind _returnvalue (UserInterface|CreateWidget "/Game/UI/WBP_PauseMenu.WBP_PauseMenu_C" self))
  (bind _output_get (Variables|Default|SetCurrentPauseMenu _returnvalue))
  (UserInterface|Viewport|AddtoViewport _returnvalue 0)
  (Variables|Default|SetbShowMouseCursor _self true)
  (Input|SetInputModeGameandUI _self _output_get "DoNotLock" true))

(fn UpdateNewKey
  (bind _result (Math|Integer|DecrementInt (Variables|Default|GetKeysToGather))
    (:%20%20
      (Default|EquipKey (Variables|Default|GetPlayerHUD) _result)
      ;[1 1 1] Do we have all the keys?
      (if (<= _result 0)
        ;[1 1 1] Set objective text to find exit
        (Default|SetObjectiveText (Variables|Default|GetPlayerHUD) (Utilities|Text|ToText(String) "Find The Exit And Escape!"))))))