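; BP_PlayerChar is the player character, handling movement, look, jump and crouch input along with health, damage and death.
; AddDamage lowers health and plays a hurt sound, or on death disables mesh collision, stops the heartbeat and triggers game over.
; Health bar updates, key pickups and game over are routed through BP_PlayerController.
; SetHeartBeatSound fades a heartbeat audio component in or out on request.
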(event Input|ActionEvents|InputActionJump
  (params (Key :type Key%20Structure :default "None"))
  ;[1 1 1] Movement Inputs
  (:Pressed
    (Character|Jump))
  (:Released
    (Character|StopJumping)))

(event Input|ActionEvents|InputActionCrouch
  (params (Key :type Key%20Structure :default "None"))
  ;[1 1 1] Movement Inputs
  (:Pressed
    (Character|Crouch))
  (:Released
    (Character|UnCrouch)))

(event Input|AxisEvents|InputAxisMoveForward
  (params (AxisValue :type Float%20%28single-precision%29))
  ;[1 1 1] Movement Inputs
  (Pawn|Input|AddMovementInput (Transformation|GetActorForwardVector) AxisValue false))

(event Input|AxisEvents|InputAxisMoveRight
  (params (AxisValue :type Float%20%28single-precision%29))
  ;[1 1 1] Movement Inputs
  (Pawn|Input|AddMovementInput (Transformation|GetActorRightVector) AxisValue false))

(event Input|AxisEvents|InputAxisLookUp
  (params (AxisValue :type Float%20%28single-precision%29))
  ;[1 1 1] Movement Inputs
  (Pawn|Input|AddControllerPitchInput AxisValue))

(event Input|AxisEvents|InputAxisTurn
  (params (AxisValue :type Float%20%28single-precision%29))
  ;[1 1 1] Movement Inputs
  (Pawn|Input|AddControllerYawInput AxisValue))

(fn ConstructionScript)

(fn AddDamage
  (params (DamageAmount :type Float%20%28single-precision%29))
  ;[1 1 1] Check if health <= 0
  (if (<= (- (Variables|Default|GetPlayerHealth) DamageAmount) 0.0)
    (Variables|Default|SetPlayerHealth 0.0)
    (CallFunction|UpdateHealthBar)
    (Variables|Default|SetbDied true)
    (Collision|SetCollisionEnabled (Variables|Character|GetMesh) "NoCollision")
    (bind _asbp_player_controller (Utilities|Casting|CastToBP_PlayerController (Pawn|GetController))
      (:then
        (Audio|PlaySound2D "/Game/Sound/163442__under7dude__man-dying.163442__under7dude__man-dying" 1.0 1.0 0.0 0 0))
      (:CastFailed
        _))
    (Audio|Components|Audio|Stop (Variables|Default|GetHeartBeat))
    (Default|CallGameOver _asbp_player_controller false)
    (else
      (Variables|Default|SetPlayerHealth (- (Variables|Default|GetPlayerHealth) DamageAmount))
      (CallFunction|UpdateHealthBar)
      (Audio|PlaySound2D "/Game/Sound/342229__christopherderp__hurt-1-male.342229__christopherderp__hurt-1-male" 1.0 1.0 0.0 0 0))))

(fn UpdateHealthBar
  ;[1 1 1] Update health bar player HUD
  (bind _asbp_player_controller (Utilities|Casting|CastToBP_PlayerController (Pawn|GetController)))
  (Default|SetHealthPercent (Variables|/Game/Blueprints/BP_PlayerController.BP_PlayerController_C|GetPlayerHUD _asbp_player_controller) (/ (Variables|Default|GetPlayerHealth) (Variables|Default|GetMaxHealth))))

(fn PickupKey
  (bind _asbp_player_controller (Utilities|Casting|CastToBP_PlayerController (Pawn|GetController)))
  (Default|UpdateNewKey _asbp_player_controller))

(fn SetHeartBeatSound
  (params (bTurnOn :type Boolean))
  (if bTurnOn
    (if (not (Audio|Components|Audio|IsPlaying (Variables|Default|GetHeartBeat)))
      (Audio|Components|Audio|FadeIn (Variables|Default|GetHeartBeat) 1.5 1.0 0.0 :!class /Script/Engine.AudioComponent))
    (elif (Audio|Components|Audio|IsPlaying (Variables|Default|GetHeartBeat))
      (Audio|Components|Audio|FadeOut (Variables|Default|GetHeartBeat) 1.5 0.0 :!class /Script/Engine.AudioComponent))))