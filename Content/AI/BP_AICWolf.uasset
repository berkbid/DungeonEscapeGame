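; AI controller for the wolf that runs a patrol behavior tree and tracks the player through AI perception.
; On possess, it copies the wolf's patrol points and seeds the blackboard with the first, while GetNextPoint cycles through them in a loop.
; Sensing the player sets TargetActor and starts the player's heartbeat sound.
; Losing the player starts a grace timer, cancelled on re-detection, that clears both when it expires.
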(event OnTargetPerceptionUpdated(AIPerception)
  (params (Actor :type Actor%20Object%20Reference) (Stimulus :type AI%20Stimulus%20Structure))
  (bind _output_get (Variables|AI|SetSensed%20Actor Actor))
  (Utilities|Casting|CastToBP_PlayerChar _output_get)
  (if (.bsuccessfullysensed Stimulus)
    ;[1 1 1] Update we have seen player
    (Utilities|Time|ClearandInvalidateTimerbyHandle (Variables|AI|GetLostSightHandle))
    (AI|Components|Blackboard|SetValueasObject (AI|GetBlackboard 0) (Utilities|Name|MakeLiteralName "TargetActor") (Variables|AI|GetSensed%20Actor))
    (bind _asbp_player_char (Utilities|Casting|CastToBP_PlayerChar (Variables|AI|GetSensed%20Actor)))
    (Default|SetHeartBeatSound _asbp_player_char true)
    (else
      ;[1 1 1] If we lose sight of player, start a timer and drop target after timer
      (bind _returnvalue (Utilities|Time|SetTimerbyEvent (delegate Custom|LostSightOfPlayer) (Variables|AI|GetLostSightTime)))
      (Variables|AI|SetLostSightHandle _returnvalue))))

(event Custom|LostSightOfPlayer
  ;[1 1 1] If we lose sight of player, start a timer and drop target after timer
  (Utilities|IsValid (Variables|AI|GetSensed%20Actor)
    (:Is%20Valid
      (bind _asbp_player_char (Utilities|Casting|CastToBP_PlayerChar (Variables|AI|GetSensed%20Actor))
        (:then
          (Default|SetHeartBeatSound _asbp_player_char false))
        (:CastFailed
          _)))
    (:Is%20Not%20Valid
      _))
  (AI|Components|Blackboard|SetValueasObject (AI|GetBlackboard 0) (Utilities|Name|MakeLiteralName "TargetActor") 0)
  (Variables|AI|SetSensed%20Actor 0))

(event EventPossess
  (params (PossessedPawn :type Pawn%20Object%20Reference))
  (bind _asbp_aiwolf (Utilities|Casting|CastToBP_AIWolf PossessedPawn))
  (bind _output_get (Variables|AI|SetWolfArrayPoints (Variables|/Game/AI/BP_AIWolf.BP_AIWolf_C|GetArrayPoints _asbp_aiwolf)))
  (Variables|AI|SetNumPoints (Utilities|Array|Length _output_get))
  (bind _output_get_2 (Variables|AI|SetCurrentPoint 0))
  (bind _blackboardcomponent (Class|AIController|UseBlackboard "/Game/AI/BB_AIPatrol.BB_AIPatrol"))
  (AI|Components|Blackboard|SetValueasObject _blackboardcomponent (Utilities|String|StringToName (Utilities|String|MakeLiteralString "NextTargetPoint")) (Utilities|Array|Get(acopy) _output_get _output_get_2))
  (AI|RunBehaviorTree "/Game/AI/BT_AIPatrol.BT_AIPatrol"))

(fn ConstructionScript)

(fn GetNextPoint
  ;[1 1 1] Return next targetpoint in array, loop back to start after last point
  (bind _result (Math|Integer|IncrementInt (Variables|AI|GetCurrentPoint))
    (:%20%20
      (if (>= _result (Variables|AI|GetNumPoints))
        (Variables|AI|SetCurrentPoint 0))
      (return (Utilities|Array|Get(acopy) (Variables|AI|GetWolfArrayPoints) (Variables|AI|GetCurrentPoint))))))